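; Game mode for a networked test level that fills the world with collectible creatures around a TargetPoint at BeginPlay.
; Every tick it jitters the actors in ActorsToSpawn by random offsets projected onto the navmesh.
; It tracks controllers and player info on login and logout, pushing the list to GS_MultiplayerConfig after a short delay.
; Modify forwards creature collection to that game state, and PlayerinfoMod overwrites a player's stored info.
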(event `self.ReceiveBeginPlay`
  (bind _returnvalue (`GameplayStatics.GetActorOfClass` "/Script/Engine.TargetPoint"))
  (`self.FillWorld` "/Game/GamePlayDemo/BluePrints/Collectibles/BP_CollectibleCreature.BP_CollectibleCreature_C" (`self.MaxActors`) (`self.K2_GetActorLocation` _returnvalue) 3000.0)
  (`KismetSystemLibrary.Delay` 3.0))

(event `MoveNonNPS`
  (for _array_element (`self.ActorsToSpawn`)
    (`self.K2_SetActorLocation` _array_element (`NavigationSystemV1.K2_ProjectPointToNavigation` (+ (`self.K2_GetActorLocation` _array_element) (* (`KismetMathLibrary.RandomUnitVector`) (* 1000.0 (`GameplayStatics.GetWorldDeltaSeconds`)))) null null (10000.0 10000.0 10000.0)) false false)))

(event `self.ReceiveTick`
  (params (DeltaSeconds :type "Float (single-precision)"))
  (`self.MoveNonNPS`))

(event `self.K2_PostLogin`
  (params (NewPlayer :type "PlayerController Object Reference"))
  (bind _asbp_multi_player_controller (cast `/Game/GamePlayDemo/BluePrints/PlayerControllers/BP_MultiPlayerController` NewPlayer))
  (`KismetArrayLibrary.Array_Add` (`self.AllPlayers`) _asbp_multi_player_controller)
  (`KismetArrayLibrary.Array_Add` (`self.AllPlayerInfo`) (`/Game/GamePlayDemo/BluePrints/PlayerControllers/BP_MultiPlayerController.PlayerInfo` _asbp_multi_player_controller))
  (`self.UpdatePlayerList` :!label _label))

(event `self.K2_OnLogout`
  (params (ExitingController :type "Controller Object Reference"))
  (bind _asbp_multi_player_controller (cast `/Game/GamePlayDemo/BluePrints/PlayerControllers/BP_MultiPlayerController` ExitingController))
  (`KismetArrayLibrary.Array_RemoveItem` (`self.AllPlayers`) _asbp_multi_player_controller)
  (`KismetArrayLibrary.Array_RemoveItem` (`self.AllPlayerInfo`) (`/Game/GamePlayDemo/BluePrints/PlayerControllers/BP_MultiPlayerController.PlayerInfo` _asbp_multi_player_controller))
  (goto _label))

(event `UpdatePlayerList`
  (`KismetSystemLibrary.Delay` 0.5)
  (bind _asgs_multiplayer_config (cast `/Game/GamePlayDemo/BluePrints/GameStates/GS_MultiplayerConfig` (`GameplayStatics.GetGameState`)))
  (`/Game/GamePlayDemo/BluePrints/GameStates/GS_MultiplayerConfig.UpdateAllPlayers` _asgs_multiplayer_config (`self.MaxActors`) (`self.AllPlayerInfo`)))

(event `Modify`
  (params (PlayerInfo :type "/Game/GamePlayDemo/BluePrints/Structs/S_PlayerInfo Structure"))
  (bind _asgs_multiplayer_config (cast `/Game/GamePlayDemo/BluePrints/GameStates/GS_MultiplayerConfig` (`GameplayStatics.GetGameState`)))
  (`/Game/GamePlayDemo/BluePrints/GameStates/GS_MultiplayerConfig.OnCollectedCreature` _asgs_multiplayer_config PlayerInfo))

(fn `Playerinfo Mod`
  (params (PlayerInfo :type "/Game/GamePlayDemo/BluePrints/Structs/S_PlayerInfo Structure") (PlayerId :type Integer))
  (bind _output_get (set `/Game/GamePlayDemo/BluePrints/PlayerControllers/BP_MultiPlayerController.PlayerInfo` PlayerInfo (`|GetArrayItem` (`self.AllPlayers`) PlayerId)))
  (`KismetSystemLibrary.PrintString` (`KismetTextLibrary.Conv_TextToString` (break `/Game/GamePlayDemo/BluePrints/Structs/S_PlayerInfo` _output_get))))

(fn `UserConstructionScript`)