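; Multiplayer GameState that shares the player list and creature-collection info with every W_PlayerHUD widget.
; UpdateAllPlayers stores the actor maximum, copies PlayerArray into AllPlayerStates and sets PlayerInfoArray.
; The AllPlayerStates RepNotify repopulates each HUD's list.
; The PlayerInfoArray RepNotify calls OnCollectedCreature with no player info supplied, which runs ModifyCollection on each HUD.
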(event `UpdateAllPlayers`
  (params (maxActors :type Integer) (PlayerInfoArray :type "Array of /Game/GamePlayDemo/BluePrints/Structs/S_PlayerInfo Structure"))
  (set `self.Max Actors` maxActors)
  (set `self.AllPlayerStates` (`self.PlayerArray`))
  (set `self.Player Info Array` PlayerInfoArray))

(event `OnCollectedCreature`
  (params (CurrentPlayerInfo :type "/Game/GamePlayDemo/BluePrints/Structs/S_PlayerInfo Structure"))
  (bind _foundwidgets (`WidgetBlueprintLibrary.GetAllWidgetsOfClass` "/Game/GamePlayDemo/UI/W_PlayerHUD.W_PlayerHUD_C" false))
  (for _array_element _foundwidgets
    (`/Game/GamePlayDemo/UI/W_PlayerHUD.ModifyCollection` _array_element self CurrentPlayerInfo)))

(fn `OnRep_AllPlayerStates`
  (bind _foundwidgets (`WidgetBlueprintLibrary.GetAllWidgetsOfClass` "/Game/GamePlayDemo/UI/W_PlayerHUD.W_PlayerHUD_C" false))
  (for _array_element _foundwidgets
    (`/Game/GamePlayDemo/UI/W_PlayerHUD.PoplulateList` _array_element self)))

(fn `OnRep_Player Info Array`
  (`self.OnCollectedCreature` (struct)))

(fn `UserConstructionScript`)