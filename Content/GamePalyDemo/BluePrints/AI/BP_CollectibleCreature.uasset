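; BP_CollectibleCreature is a collectible creature actor that adds to a count on the game mode when collected.
; On BeginPlay it casts and caches the game mode, then binds to its own OnDestroyed event.
; Interact destroys the actor, and the destroyed handler increments the game mode's CurrentActors, so destruction by any cause while bound also counts.
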(event `self.ReceiveBeginPlay`
  (bind _asgm_networked_ability_cpptest (cast `` (`GameplayStatics.GetGameMode`)))
  (bind _output_get (set `self.GameModeRef` _asgm_networked_ability_cpptest))
  (`/Engine/EditorBlueprintResources/StandardMacros.IsValid` _output_get
    (:`Is Valid`
      (add `self.OnDestroyed` (delegate `OnDestroyed_Event`)))))

(event `OnDestroyed_Event` :!signature `self.OnDestroyed`
  (params (DestroyedActor :type "Actor Object Reference"))
  (bind _gamemoderef (`self.GameModeRef`)
    (:`then`
      (`/Engine/EditorBlueprintResources/StandardMacros.IncrementInt` (`/Game/GamePalyDemo/BluePrints/AI/BP_CollectibleCreature.currentActors` _gamemoderef)))
    (:`else`)))

(event `self.Interact`
  (`self.K2_DestroyActor`))

(fn `UserConstructionScript`)