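; Game mode for a networked ability test that populates the world with creature AI and tracks connected multiplayer controllers.
; BeginPlay calls FillWorld to spawn BP_CreatureAI around a TargetPoint, and Tick feeds each player character's location to RenderBasedOnDistance.
; Login and logout maintain AllPlayers, then after a short delay tell GS_MultiplayerConfig to update all players.
; UpdateCollection sends the collected and maximum actor counts to the indexed player's controller.
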(event `self.ReceiveBeginPlay`
  (bind _returnvalue (`GameplayStatics.GetActorOfClass` "/Script/Engine.TargetPoint"))
  (`self.FillWorld` "/Game/GamePlayDemo/BluePrints/AI/BP_CreatureAI.BP_CreatureAI_C" (`self.MaxActors`) (`self.K2_GetActorLocation` _returnvalue) 1000.0))

(event `self.ReceiveTick`
  (params (DeltaSeconds :type "Float (single-precision)"))
  (for (_ _array_index) (`self.AllPlayers`)
    (bind _returnvalue (`GameplayStatics.GetPlayerCharacter` _array_index))
    (`/Engine/EditorBlueprintResources/StandardMacros.IsValid` _returnvalue
      (:`Is Valid`
        (`self.RenderBasedOnDistance` (`self.K2_GetActorLocation` _returnvalue))))))

(event `self.K2_PostLogin`
  (params (NewPlayer :type "PlayerController Object Reference"))
  (bind _asbp_multi_player_controller (cast `/Game/GamePlayDemo/BluePrints/PlayerControllers/BP_MultiPlayerController` NewPlayer))
  (`KismetArrayLibrary.Array_Add` (`self.AllPlayers`) _asbp_multi_player_controller)
  (`self.UpdatePlayerList` :!label _label))

(event `UpdatePlayerList`
  (`KismetSystemLibrary.Delay` 0.5)
  (bind _asgs_multiplayer_config (cast `/Game/GamePlayDemo/BluePrints/GameStates/GS_MultiplayerConfig` (`GameplayStatics.GetGameState`)))
  (`/Game/GamePlayDemo/BluePrints/GameStates/GS_MultiplayerConfig.UpdateAllPlayers` _asgs_multiplayer_config))

(event `self.K2_OnLogout`
  (params (ExitingController :type "Controller Object Reference"))
  (bind _asbp_multi_player_controller (cast `/Game/GamePlayDemo/BluePrints/PlayerControllers/BP_MultiPlayerController` ExitingController))
  (`KismetArrayLibrary.Array_RemoveItem` (`self.AllPlayers`) _asbp_multi_player_controller)
  (goto _label))

(fn `UpdateCollection`
  (params (PlayerId :type Integer))
  (`/Game/GamePlayDemo/BluePrints/PlayerControllers/BP_MultiPlayerController.OC_UpdateCollectedCount` (`|GetArrayItem` (`self.AllPlayers`) PlayerId) (`self.CollectedActors`) (`self.MaxActors`)))

(fn `UserConstructionScript`)