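; Player controller for the networked ability test game mode that tracks how many items its player has collected.
; BeginPlay caches the GM_NetworkedAbilityTest reference, then runs a delay that leads to nothing.
; OC_UpdateCollectedCount increments the count in the PlayerInfo struct and passes it to the game mode's Modify when that reference is valid.
; SetupUI adds the W_PlayerHUD widget to the viewport, and TranferPlayerInfo returns a zero count with Max; neither is called here.
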(event `self.ReceiveBeginPlay`
  (bind _asgm_networked_ability_test (cast `/Game/GamePlayDemo/BluePrints/NewGameMode/GM_NetworkedAbilityTest` (`GameplayStatics.GetGameMode`)))
  (set `self. GameModeRef` _asgm_networked_ability_test)
  (`KismetSystemLibrary.Delay` 3.0))

(event `OC_UpdateCollectedCount`
  (bind (_playername _id _collected) (break `/Game/GamePlayDemo/BluePrints/Structs/S_PlayerInfo` (`self.PlayerInfo`)))
  (bind _result (`/Engine/EditorBlueprintResources/StandardMacros.IncrementInt` _collected)
    (:`  `
      (bind _output_get (set `self.PlayerInfo` (make `/Game/GamePlayDemo/BluePrints/Structs/S_PlayerInfo` _playername _id _result)))
      (bind __gamemoderef (`self. GameModeRef`)
        (:`then`
          (`/Game/GamePlayDemo/BluePrints/NewGameMode/GM_NetworkedAbilityTest.Modify` __gamemoderef _output_get))
        (:`else`)))))

(fn `SetupUI`
  (bind _returnvalue (`|CreateWidget` "/Game/GamePlayDemo/UI/W_PlayerHUD.W_PlayerHUD_C" self))
  (`/Engine/EditorBlueprintResources/StandardMacros.IsValid` _returnvalue
    (:`Is Valid`
      (`UserWidget.AddToViewport` _returnvalue 0))))

(fn `TranferPlayerInfo`
  (returns (collected :type Integer) (max :type Integer))
  (return 0 (`self.Max`)))

(fn `UserConstructionScript`)