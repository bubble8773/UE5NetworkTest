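; Game mode that fills the level with SimpleAI actors, shows only those near the player and handles the win condition.
; BeginPlay calls FillWorld around the first TargetPoint; Tick re-scans all SimpleAI, hiding any beyond a fixed distance from the last logged-in player's character.
; Tick also runs WinLose, which freezes time and prints a win message once GetCurrentActorP equals MaxActors.
; The UpdateStats destroy handler is empty and never bound.
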(event `self.K2_PostLogin`
  (params (NewPlayer :type "PlayerController Object Reference"))
  (set `self.CurrentPlayerIndex` (`GameplayStatics.GetPlayerControllerID` NewPlayer)))

(event `self.ReceiveBeginPlay`
  (bind _outactors (`GameplayStatics.GetAllActorsOfClass` "/Script/Engine.TargetPoint"))
  (bind _returnvalue_location (`KismetMathLibrary.BreakTransform` (`self.GetTransform` (`|GetArrayItem` _outactors))))
  (`self.FillWorld` "/Game/GamePlayDemo/BluePrints/AI/SimpleAI.SimpleAI_C" (`self.maxActors`) _returnvalue_location 1000.0)
  (bind _outactors_2 (`GameplayStatics.GetAllActorsOfClass` "/Game/GamePlayDemo/BluePrints/AI/SimpleAI.SimpleAI_C" :!label _label))
  (for _array_element _outactors_2
    (`self.RenderBasedOnDistance` (`self.K2_GetActorLocation` (`GameplayStatics.GetPlayerCharacter` (`self.CurrentPlayerIndex`))) _array_element 1000.0)))

(event `UpdateStats` :!signature `self.OnDestroyed`
  (params (DestroyedActor :type "Actor Object Reference"))
  ;[1 1 1] Using destry
)

(event `self.ReceiveTick`
  (params (DeltaSeconds :type "Float (single-precision)"))
  (`self.WinLose`)
  (`/Engine/EditorBlueprintResources/StandardMacros.IsValid` (`GameplayStatics.GetPlayerCharacter` (`self.CurrentPlayerIndex`))
    (:`Is Valid`
      (goto _label))))

(fn `RenderBasedOnDistance`
  (params (PlayerLocation :type "Vector Structure") (Collectible :type "Actor Object Reference") (DistanceCheck :type "Float (double-precision)"))
  (`self.SetActorHiddenInGame` (`local.Collectible`) (> (`KismetMathLibrary.Vector_Distance` PlayerLocation (`self.K2_GetActorLocation` Collectible)) DistanceCheck)))

(fn `UserConstructionScript`)

(fn `WinLose`
  (bind _returnvalue (`self.GetCurrentActor_p`))
  (if (== (`self.maxActors`) _returnvalue)
    (`GameplayStatics.SetGlobalTimeDilation` 0.0)
    (`KismetSystemLibrary.PrintString` "U Won")))