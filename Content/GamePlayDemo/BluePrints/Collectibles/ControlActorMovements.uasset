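; Controller Blueprint that randomly jitters CollectMe collectible actors around the level.
; Shortly after BeginPlay it caches all CollectMe actors in an array.
; Tick, throttled by a Delay, applies a random horizontal world offset to one of the first three, re-rolling the index between validity check and move.
; An unconnected alternative branch would send actors to random reachable navigation points and rotate them with look-at rotation.
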(event `self.ReceiveBeginPlay`
  (`KismetSystemLibrary.Delay` 0.2)
  (bind _outactors (`GameplayStatics.GetAllActorsOfClass` "/Game/GamePlayDemo/BluePrints/Collectibles/CollectMe.CollectMe_C"))
  (set `self.Out Actors` _outactors))

(event `self.ReceiveTick`
  (params (DeltaSeconds :type "Float (single-precision)"))
  (bind _output (`|GetArrayItem` (`self.Out Actors`) (`KismetMathLibrary.RandomIntegerInRange` 0 2)))
  (bind (_returnvalue_x _returnvalue_y) (`KismetMathLibrary.BreakVector` (* 50.0 (`KismetMathLibrary.RandomUnitVector`))))
  (`KismetSystemLibrary.Delay` 1.0)
  (`/Engine/EditorBlueprintResources/StandardMacros.IsValid` _output
    (:`Is Valid`
      (`SceneComponent.K2_AddWorldOffset` (`Actor.RootComponent` _output) (`KismetMathLibrary.MakeVector` _returnvalue_x _returnvalue_y 0.0) false false)
      (`KismetSystemLibrary.Delay` 1.0))))

(fn `UserConstructionScript`)